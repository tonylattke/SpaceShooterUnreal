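; Ghost actor that replays a path of positions from GhostInfo, handed over with a player reference through Initialize.
; Each Tick teleports it to the next stored location without sweeping, so playback speed follows frame rate rather than time.
; When the locations run out, it calls GhostReportTimesUp on the player and destroys itself.
; A separate Shoot function spawns SelectedAmmo at the BulletSpawner location with zero rotation.
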(event EventBeginPlay)

(event Collision|EventActorBeginOverlap
  (params (OtherActor :type Actor%20Object%20Reference)))

(event EventTick
  (params (DeltaSeconds :type Float%20%28single-precision%29))
  (bind _locations (Variables|Default|GetLocations))
  (if (Utilities|Array|IsNotEmpty _locations)
    (if (< (Variables|Default|GetCurrentLocationIndex) (Variables|Default|GetNumberOfLocations))
      (Transformation|SetActorLocation (Utilities|Array|Get(acopy) _locations (Variables|Default|GetCurrentLocationIndex)) false false)
      (Math|Integer|IncrementInt (Variables|Default|GetCurrentLocationIndex))
      (else
        (Default|GhostReportTimesUp (Variables|Default|GetPlayerRef) self)
        (Actor|DestroyActor)))))

(fn ConstructionScript)

(fn Initialize
  (params (GhostInfo :type ST%20Ghost%20Info%20Structure) (PlayerRef :type BP%20Player%20Object%20Reference))
  (Variables|Default|SetPlayerRef PlayerRef)
  (bind _output_get (Variables|Default|SetLocations (Utilities|Struct|BreakST_GhostInfo GhostInfo)))
  (Variables|Default|SetNumberOfLocations (Utilities|Array|Length _output_get)))

(fn Shoot
  (Game|SpawnActorfromClass (Variables|Default|GetSelectedAmmo) (Math|Transform|MakeTransform (Transformation|GetWorldLocation (Variables|Default|GetBulletSpawner))) "Undefined" "MultiplyWithRoot" 0 0))