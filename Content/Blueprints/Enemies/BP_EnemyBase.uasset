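; Base enemy actor that moves every tick along MovementDirection at Speed and loses a life point when its Box overlaps a BP_BaseShoot.
; At zero life it reports to the game mode passed in through Initalize, then destroys itself.
; DirectionChnager picks a random diagonal XY heading, though nothing here calls it.
; Ammo helpers cap CurrentAmmo against AvailableAmmo, but the bullet spawn and shot sound are unwired in this graph.
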(event OnComponentBeginOverlap(Box)
  (params (OverlappedComponent :type Primitive%20Component%20Object%20Reference) (OtherActor :type Actor%20Object%20Reference) (OtherComp :type Primitive%20Component%20Object%20Reference) (OtherBodyIndex :type Integer) (bFromSweep :type Boolean) (SweepResult :type Hit%20Result%20Structure%20%28by%20ref%29))
  (Utilities|Casting|CastToBP_BaseShoot OtherActor)
  (Math|Integer|DecrementInt (Variables|Default|GetLifePoints)
    (:%20%20
      (if (<= (Variables|Default|GetLifePoints) 0)
        (CallFunction|DestoyandReport)))))

(event EventBeginPlay)

(event EventTick
  (params (DeltaSeconds :type Float%20%28single-precision%29))
  (Transformation|SetActorLocation (+ (Transformation|GetActorLocation) (* DeltaSeconds (Variables|Default|GetMovementDirection) (Variables|Default|GetSpeed))) false false))

(fn ConstructionScript)

(fn SetupController)

(fn AmmoDie
  (Variables|Default|SetCurrentAmmo (- (Variables|Default|GetCurrentAmmo) 1)))

(fn CanShoot
  (return (< (Variables|Default|GetCurrentAmmo) (Variables|Default|GetAvailableAmmo))))

(fn Initalize
  (params (MyGameMode :type BP%20Game%20Mode%20Object%20Reference))
  (Variables|Default|SetMyGameMode MyGameMode))

(fn DestoyandReport
  (Default|DestroyEnemy (Variables|Default|GetMyGameMode) self)
  (Actor|DestroyActor))

(fn DirectionChnager
  (Utilities|FlowControl|Sequence
    (:then_0
      (if (< (Math|Random|RandomFloat) 0.5)
        (LocalVariables|SetAxisX -1.0)
        (else
          (LocalVariables|SetAxisX 1.0))))
    (:then_1
      (if (< (Math|Random|RandomFloat) 0.5)
        (LocalVariables|SetAxisY -1.0)
        (else
          (LocalVariables|SetAxisY 1.0))))
    (:then_2
      (Variables|Default|SetMovementDirection (Math|Vector|MakeVector (LocalVariables|GetAxisX) (LocalVariables|GetAxisY) 0.0)))))