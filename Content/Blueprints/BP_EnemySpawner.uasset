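; BP_EnemySpawner is a moving spawn point that creates enemies of its configured class at its own transform.
; On BeginPlay it registers itself in BP_GameMode's spawner collection, and every tick it moves along MovementDirection at Speed.
; SpawnEnemy initializes each new BP_EnemyBase with the game mode and returns it, while ChangeDirection reverses movement; neither is called within this Blueprint.
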(event EventBeginPlay
  ;[1 1 1] Self register in game mode
  (bind _asbp_game_mode (Utilities|Casting|CastToBP_GameMode (Game|GetGameMode)))
  (bind _output_get (Variables|Default|SetBPGameMode _asbp_game_mode))
  (Utilities|Array|Add (Variables|/Game/Blueprints/BP_GameMode.BP_GameMode_C|GetEnemySpawnerCollection _output_get) self))

(event EventTick
  (params (DeltaSeconds :type Float%20%28single-precision%29))
  (CallFunction|UpdateActorLocation self DeltaSeconds (Variables|Default|GetMovementDirection) (Variables|Default|GetSpeed)))

(fn ConstructionScript)

(fn SpawnEnemy
  (bind _returnvalue (Game|SpawnActorfromClass (Variables|Default|GetEnemyClass) (Transformation|GetActorTransform) "Undefined" "MultiplyWithRoot" 0 0))
  (bind _asbp_enemy_base (Utilities|Casting|CastToBP_EnemyBase _returnvalue))
  (Default|Initalize _asbp_enemy_base (Variables|Default|GetBPGameMode))
  (return _returnvalue))

(fn ChangeDirection
  (Variables|Default|SetMovementDirection (* (Variables|Default|GetMovementDirection) -1.0)))