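; BP_SimpleShot is a simple projectile used as player ammo.
; Each tick it moves along world +X at a constant speed by setting its location directly, without sweeping for collision.
; After a fixed delay from BeginPlay it calls AmmoDie on its Master reference and destroys itself.
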(event EventBeginPlay
  (Utilities|FlowControl|Delay 2.0)
  (Default|AmmoDie (Variables|Default|GetMaster))
  (Actor|DestroyActor))

(event Collision|EventActorBeginOverlap
  (params (OtherActor :type Actor%20Object%20Reference)))

(event EventTick
  (params (DeltaSeconds :type Float%20%28single-precision%29))
  (bind _returnvalue (Transformation|GetActorLocation))
  (bind (_x _y _z) (Math|Vector|BreakVector _returnvalue))
  (Transformation|SetActorLocation (Math|Vector|MakeVector (+ (* DeltaSeconds 5e+02) _x) _y _z) false false))

(fn ConstructionScript
  (|CallParentFunction))