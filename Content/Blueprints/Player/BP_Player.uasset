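; Player pawn for a shooter in which recorded "souls" return as ghosts that fire alongside the player.
; Enhanced Input drives movement clamped to game mode ranges, pausing, and shooting limited by a live-projectile count.
; Tick records locations; a simulated-death key banks that path, and another spawns a BP_Ghost from the oldest one.
; Shots propagate to active ghosts, while enemy overlaps notify the game mode and spawn hit effects.
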(event OnComponentBeginOverlap(CollisionBox)
  (params (OverlappedComponent :type Primitive%20Component%20Object%20Reference) (OtherActor :type Actor%20Object%20Reference) (OtherComp :type Primitive%20Component%20Object%20Reference) (OtherBodyIndex :type Integer) (bFromSweep :type Boolean) (SweepResult :type Hit%20Result%20Structure%20%28by%20ref%29))
  (bind _mygamemode (Variables|Default|GetMyGameMode))
  (bind _asbp_enemy_base (Utilities|Casting|CastToBP_EnemyBase OtherActor))
  (Utilities|IsValid _mygamemode
    (:Is%20Valid
      (Default|HitPlayer _mygamemode _asbp_enemy_base)
      (Niagara|SpawnSystematLocation "/Game/VFX/NS_Hit.NS_Hit" (Transformation|GetActorLocation _asbp_enemy_base)))))

(event Input|EnhancedActionEvents|EnhancedInputActionIA_Shoot
  (params (ActionValue :type Boolean) (ElapsedSeconds :type Float%20%28double-precision%29) (TriggeredSeconds :type Float%20%28double-precision%29) (InputAction :type Input%20Action%20Object%20Reference :default "/Game/Blueprints/Input/IA_Shoot.IA_Shoot"))
  (:Completed
    (if (CallFunction|CanShoot)
      (Math|Integer|IncrementInt (Variables|Default|GetCurrentAmmo)
        (:%20%20
          (bind _returnvalue (Game|SpawnActorfromClass (Variables|Default|GetSelectedAmmo) (Math|Transform|MakeTransform (Transformation|GetWorldLocation (Variables|Default|GetBulletSpawner))) "Undefined" "MultiplyWithRoot" 0 0))
          (Variables|/Game/Blueprints/Player/Ammo/BP_BaseShoot.BP_BaseShoot_C|SetMaster _returnvalue self)
          (Audio|PlaySound2D "/Game/Sounds/S_SimpleShot.S_SimpleShot" 1.0 1.0 0.0 0 0)
          (for _array_element (Variables|Default|GetMyGhosts)
            (Utilities|IsValid _array_element
              (:Is%20Valid
                (Default|Shoot _array_element)))))))))

(event Input|EnhancedActionEvents|EnhancedInputActionIA_Move
  (params (ActionValue :type Vector%202D%20Structure) (ElapsedSeconds :type Float%20%28double-precision%29) (TriggeredSeconds :type Float%20%28double-precision%29) (InputAction :type Input%20Action%20Object%20Reference :default "/Game/Blueprints/Input/IA_Move.IA_Move"))
  (CallFunction|UpdateLocation ActionValue ElapsedSeconds))

(event Input|EnhancedActionEvents|EnhancedInputActionIA_Pause
  (params (ActionValue :type Boolean) (ElapsedSeconds :type Float%20%28double-precision%29) (TriggeredSeconds :type Float%20%28double-precision%29) (InputAction :type Input%20Action%20Object%20Reference :default "/Game/Blueprints/Input/IA_Pause.IA_Pause"))
  (:Completed
    (bind _asbp_game_mode (Utilities|Casting|CastToBP_GameMode (Game|GetGameMode)))
    (Default|HandlePause _asbp_game_mode)))

(event EventBeginPlay
  (CallFunction|SetupController)
  (bind _asbp_game_mode (Utilities|Casting|CastToBP_GameMode (Game|GetGameMode)))
  (Variables|Default|SetMyGameMode _asbp_game_mode))

(event Collision|EventActorBeginOverlap
  (params (OtherActor :type Actor%20Object%20Reference)))

(event EventTick
  (params (DeltaSeconds :type Float%20%28single-precision%29))
  (CallFunction|SaveCurrentLocation))

(event Input|KeyboardEvents|LeftCtrl
  (params (Key :type Key%20Structure :default "None"))
  (bind _ghostsavailabletospawn (Variables|Default|GetGhostsAvailableToSpawn))
  (:Pressed
    (if (Utilities|Array|IsEmpty (Variables|Default|GetGhostsAvailableToSpawn))
      (Development|PrintString "No souls avilable")
      (else
        (bind _returnvalue (Game|SpawnActorfromClass "/Game/Blueprints/BP_Ghost.BP_Ghost_C" (Math|Transform|MakeTransform "0, 0, 0") "Undefined" "MultiplyWithRoot" 0 0))
        (Default|Initialize _returnvalue (Utilities|Array|Get(acopy) _ghostsavailabletospawn) self)
        (Utilities|Array|RemoveIndex _ghostsavailabletospawn)
        (Utilities|Array|Add (Variables|Default|GetMyGhosts) _returnvalue)))))

(event Input|KeyboardEvents|LeftAlt
  (params (Key :type Key%20Structure :default "None"))
  ;[1 1 1] Kill
  (:Pressed
    (Variables|Default|SetIsDead true)
    (CallFunction|BackupCurrentSoul)
    (Variables|Default|SetIsDead false)))

(fn ConstructionScript)

(fn SetupController
  (bind _asplayer_controller (Utilities|Casting|CastToPlayerController (Pawn|GetController)))
  (Input|AddMappingContext (PlayerController|LocalPlayerSubsystems|GetEnhancedInputLocalPlayerSubsystem _asplayer_controller) "/Game/Blueprints/Input/IMC_Player.IMC_Player" 0 "(bIgnoreAllPressedKeysUntilRelease=True,bForceImmediately=False,bNotifyUserSettings=False)"))

(fn UpdateLocation
  (params (VectorInput :type Vector%202D%20Structure) (Deltatime :type Float%20%28double-precision%29))
  (bind _returnvalue (Transformation|GetActorLocation))
  (bind (_x _y) (Math|Vector2D|BreakVector2D VectorInput))
  (bind (_x_2 _y_2 _z) (Math|Vector|BreakVector _returnvalue))
  ;[1 1 1] X axis
  (LocalVariables|SetResultedX (CallFunction|CalculateNewValueinAxis _x_2 _x Deltatime (Variables|/Game/Blueprints/BP_GameMode.BP_GameMode_C|GetRangeX (Variables|Default|GetMyGameMode))))
  ;[1 1 1] Y axis
  (LocalVariables|SetResultedY (CallFunction|CalculateNewValueinAxis _y_2 _y Deltatime (Variables|/Game/Blueprints/BP_GameMode.BP_GameMode_C|GetRangeY (Variables|Default|GetMyGameMode))))
  ;[1 1 1] Z axis
  (LocalVariables|SetResultedZ _z)
  (Transformation|SetActorLocation (Math|Vector|MakeVector (LocalVariables|GetResultedX) (LocalVariables|GetResultedY) (LocalVariables|GetResultedZ)) false true)
  (return))

(fn CalculateNewValueinAxis
  (params (CurrentLocationInAxis :type Float%20%28double-precision%29) (AxisInput :type Float%20%28double-precision%29) (Deltatime :type Float%20%28double-precision%29) (Range :type Vector%202D%20Structure))
  (bind (_x _y) (Math|Vector2D|BreakVector2D Range))
  (return (Math|Float|Clamp(Float) (+ CurrentLocationInAxis (* AxisInput Deltatime (Variables|Default|GetMovementSpeed))) _x _y)))

(fn AmmoDie
  (Variables|Default|SetCurrentAmmo (- (Variables|Default|GetCurrentAmmo) 1)))

(fn CanShoot
  (return (< (Variables|Default|GetCurrentAmmo) (Variables|Default|GetAvailableAmmo))))

(fn SaveCurrentLocation
  (if (not (Variables|Default|GetIsDead))
    (Utilities|Array|Add (Variables|Default|GetCurrentGhostLocationCollector) (Transformation|GetActorLocation))))

(fn BackupCurrentSoul
  ;[1 1 1] Copy current soul locations
  (bind _copyghostlocations (CallFunction|CopyVectorArray))
  (Utilities|Array|Add (Variables|Default|GetGhostsAvailableToSpawn) (Utilities|Struct|MakeST_GhostInfo _copyghostlocations))
  ;[1 1 1] Clean current soul locations
  (Utilities|Array|Clear (Variables|Default|GetCurrentGhostLocationCollector)))

(fn CopyVectorArray
  (for _array_element (Variables|Default|GetCurrentGhostLocationCollector)
    (Utilities|Array|Add (LocalVariables|GetLocationsCopy) (|Copy _array_element)))
  (return (LocalVariables|GetLocationsCopy)))

(fn GhostReportTimesUp
  (params (CurrentGhost :type BP%20Ghost%20Object%20Reference))
  (Utilities|Array|RemoveItem (Variables|Default|GetMyGhosts) CurrentGhost))